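; Coin pickup actor for a runner game that adds one coin to the third-person game mode and then destroys itself.
; Touching the coin collects it directly unless it is already being attracted.
; When a character with an active magnet enters the outer sphere, a timeline lerps the coin mesh toward the character's mesh, then awards the coin when it finishes.
; A Collected flag prevents double counting during attraction.
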(event `self.ReceiveBeginPlay`
  (bind _asthird_person_game_mode (cast `/Game/ThirdPersonBP/Blueprints/ThirdPersonGameMode` (`GameplayStatics.GetGameMode`)))
  (set `self.GameModeRef` _asthird_person_game_mode))

(event `self.Sphere.OnComponentBeginOverlap`
  (params (OverlappedComponent :type "PrimitiveComponent Object Reference") (OtherActor :type "Actor Object Reference") (OtherComp :type "PrimitiveComponent Object Reference") (OtherBodyIndex :type Integer) (bFromSweep :type Boolean) (SweepResult :type "HitResult Structure (by ref)"))
  (bind _asthird_person_character (cast `/Game/ThirdPersonBP/Blueprints/ThirdPersonCharacter` OtherActor))
  (if (`/Game/ThirdPersonBP/Blueprints/ThirdPersonCharacter.IsMagnetActive?` _asthird_person_character)
    (set `self.Collected?` true)
    (bind (_direction _distance__normalised_) (`Timeline|Attraction` :!via `PlayFromStart`)
      (:`Update`
        (`SceneComponent.K2_SetWorldLocation` (`self.Coin`) (`KismetMathLibrary.VLerp` (`SceneComponent.K2_GetComponentLocation` (`self.Coin`)) (`SceneComponent.K2_GetComponentLocation` (`Character.Mesh` _asthird_person_character)) _distance__normalised_) false false))
      (:`Finished`
        (`/Game/ThirdPersonBP/Blueprints/ThirdPersonGameMode.AddCoins` (`self.GameModeRef`) 1)
        (`self.K2_DestroyActor`)))))

(event `self.Coin.OnComponentBeginOverlap`
  (params (OverlappedComponent :type "PrimitiveComponent Object Reference") (OtherActor :type "Actor Object Reference") (OtherComp :type "PrimitiveComponent Object Reference") (OtherBodyIndex :type Integer) (bFromSweep :type Boolean) (SweepResult :type "HitResult Structure (by ref)"))
  (cast `/Game/ThirdPersonBP/Blueprints/ThirdPersonCharacter` OtherActor)
  (if (not (`self.Collected?`))
    (bind _asthird_person_game_mode (cast `/Game/ThirdPersonBP/Blueprints/ThirdPersonGameMode` (`GameplayStatics.GetGameMode`)))
    (`/Game/ThirdPersonBP/Blueprints/ThirdPersonGameMode.AddCoins` _asthird_person_game_mode 1)
    (`self.K2_DestroyActor`)))

(fn `UserConstructionScript`)